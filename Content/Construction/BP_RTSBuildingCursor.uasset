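; BP_RTSBuildingCursor is the placement preview actor for RTS construction, showing a building mesh and an optional grid overlay.
; Setter events assign either a static or skeletal mesh with a relative transform, and a validity event swaps every material slot to a valid or invalid material.
; Each tick, it toggles the grid plane, scales it to grid size and cell size, and feeds the grid texture into a dynamic material instance.
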(event `self.ReceiveBeginPlay`
  (bind _returnvalue (`KismetMaterialLibrary.CreateDynamicMaterialInstance` (`self.GridMaterial`)))
  (bind _output_get (set `self.GridMaterialInstance` _returnvalue))
  (`PrimitiveComponent.SetMaterial` (`self.GridPlane`) 0 _output_get))

(event `self.ReceiveTick`
  (params (DeltaSeconds :type "Float (single-precision)"))
  (bind _returnvalue (* (`self.GetGridWidthAndHeight`) (/ (`self.GetGridCellSize`) 100.0)))
  (`SceneComponent.SetVisibility` (`self.GridPlane`) (`self.HasGrid`) false)
  (if (`self.HasGrid`)
    (`SceneComponent.SetRelativeScale3D` (`self.GridPlane`) (`KismetMathLibrary.MakeVector` _returnvalue _returnvalue 1.0))
    (`MaterialInstanceDynamic.SetTextureParameterValue` (`self.GridMaterialInstance`) "GridTexture" (`self.GetGridTexture`))))

(event `self.SetStaticMesh`
  (params (BuildingMesh :type "StaticMesh Object Reference") (RelativeTransform :type "Transform Structure (by ref)"))
  (`/Engine/EditorBlueprintResources/StandardMacros.IsValid` BuildingMesh
    (:`Is Valid`
      (`SceneComponent.K2_SetRelativeTransform` (`self.StaticMesh`) RelativeTransform false true)
      (`StaticMeshComponent.SetStaticMesh` (`self.StaticMesh`) BuildingMesh))))

(event `self.SetSkeletalMesh`
  (params (BuildingMesh :type "SkeletalMesh Object Reference") (RelativeTransform :type "Transform Structure (by ref)"))
  (`/Engine/EditorBlueprintResources/StandardMacros.IsValid` BuildingMesh
    (:`Is Valid`
      (`SceneComponent.K2_SetRelativeTransform` (`self.SkeletalMesh`) RelativeTransform false true)
      (`SkinnedMeshComponent.SetSkinnedAssetAndUpdate` (`self.SkeletalMesh`) BuildingMesh true))))

(event `self.SetLocationValid`
  (params (bValid :type Boolean))
  (bind _skeletalmesh (`self.SkeletalMesh`))
  (bind _staticmesh (`self.StaticMesh`))
  (bind _returnvalue (select `bool` bValid :`false` (`self.InvalidMaterial`) :`true` (`self.ValidMaterial`)))
  (`/Engine/EditorBlueprintResources/StandardMacros.IsValid` (`StaticMeshComponent.StaticMesh` (`self.StaticMesh`))
    (:`Is Valid`
      (for _index (range (`PrimitiveComponent.GetNumMaterials` _staticmesh))
        (`PrimitiveComponent.SetMaterial` _staticmesh _index _returnvalue)))
    (:`Is Not Valid`
      (for _index_2 (range (`PrimitiveComponent.GetNumMaterials` _skeletalmesh))
        (`PrimitiveComponent.SetMaterial` _skeletalmesh _index_2 _returnvalue)))))

(fn `UserConstructionScript`)