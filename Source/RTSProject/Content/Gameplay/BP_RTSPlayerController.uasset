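; RTS player controller Blueprint that owns the in-game HUD and keeps it in sync with gameplay state.
; On BeginPlay it creates WBP_IngameUI for local controllers only and adds it to the viewport.
; Selection changes and resource updates from PlayerResourcesComponent are forwarded to that widget, guarded by validity checks.
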(event `self.ReceiveBeginPlay`
  (`self.SetupIngameUI`))

(event `self.ReceiveOnSelectionChanged`
  (params (Selection :type "Array of Actor Object Reference (by ref)"))
  (bind _ingameui (`self.IngameUI`))
  (`/Engine/EditorBlueprintResources/StandardMacros.IsValid` _ingameui
    (:`Is Valid`
      (`/Game/UI/Widgets/WBP_IngameUI.SetSelectedActors` _ingameui Selection))))

(event `self.PlayerResourcesComponent.OnResourcesChanged`
  (params (ResourceType :type "RTSResourceType Class Reference") (OldResourceAmount :type "Float (single-precision)") (NewResourceAmount :type "Float (single-precision)") (bSyncedFromServer :type Boolean))
  (bind _ingameui (`self.IngameUI`))
  (`/Engine/EditorBlueprintResources/StandardMacros.IsValid` _ingameui
    (:`Is Valid`
      (`/Game/UI/Widgets/WBP_IngameUI.SetResources` _ingameui ResourceType NewResourceAmount))))

(fn `SetupIngameUI`
  (if (`self.IsLocalPlayerController`)
    (bind _returnvalue (`|CreateWidget` "/Game/UI/Widgets/WBP_IngameUI.WBP_IngameUI_C" self))
    (bind _output_get (set `self.IngameUI` _returnvalue))
    (`UserWidget.AddToViewport` _output_get 0)))

(fn `UserConstructionScript`)